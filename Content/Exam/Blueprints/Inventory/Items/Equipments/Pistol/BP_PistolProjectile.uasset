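; BP_PistolProjectile is the pistol's bullet projectile, built to be reused from a pool instead of destroyed.
; On applying damage it runs the parent logic, then disables its sphere collision and zeroes its movement velocity.
; It then adds itself back to the PistolComponent's BulletsPool and teleports to that component owner's location.
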(fn `ApplyDamage`
  (params (DamagedActor :type "Actor Object Reference"))
  (`parent.ApplyDamage` DamagedActor)
  (`PrimitiveComponent.SetCollisionEnabled` (`self.Sphere`) "NoCollision")
  (set `MovementComponent.Velocity` (0.0 0.0 0.0) (`self.ProjectileMovement`))
  (`KismetArrayLibrary.Array_Add` (`/Game/Exam/Blueprints/Inventory/Items/Equipments/Pistol/BP_PistolComponent.BulletsPool` (`self.PistolComponent`)) self)
  (`self.K2_SetActorLocation` (`self.K2_GetActorLocation` (`ActorComponent.GetOwner` (`self.PistolComponent`))) false true))

(fn `UserConstructionScript`
  (`parent.UserConstructionScript`))