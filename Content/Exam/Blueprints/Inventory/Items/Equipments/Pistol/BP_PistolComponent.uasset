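; BP_PistolComponent is a pistol equipment component that fires projectiles when executed while any BP_Enemy exists.
; With an empty BulletsPool, it spawns a BP_PistolProjectile at the owner, yawed toward the nearest enemy, with the owner pawn as instigator and itself as the projectile's component reference.
; Otherwise it removes the first pool entry, then re-enables collision and sets a fixed velocity on index 0, without repositioning or re-aiming.
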(fn `Execute`
  (locals (RandomYaw :type "Float (double-precision)"))
  (bind _bulletspool (`self.BulletsPool`))
  (bind _returnvalue_location (`KismetMathLibrary.BreakTransform` (`Actor.GetTransform` (`self.GetOwner`))))
  (bind _output (`|GetArrayItem` _bulletspool))
  (`parent.Execute`)
  (bind _outactors (`GameplayStatics.GetAllActorsOfClass` "/Game/Exam/Blueprints/Gameplay/BP_Enemy.BP_Enemy_C"))
  (if (`KismetArrayLibrary.Array_IsNotEmpty` _outactors)
    (bind _aspawn (cast `Pawn` (`self.GetOwner`)))
    (if (`KismetArrayLibrary.Array_IsEmpty` _bulletspool)
      (bind (_returnvalue_roll _returnvalue_pitch _returnvalue_yaw) (`KismetMathLibrary.BreakRotator` (`KismetMathLibrary.FindLookAtRotation` _returnvalue_location (`Actor.K2_GetActorLocation` (`.ReturnValue` (`GameplayStatics.FindNearestActor` _returnvalue_location _outactors))))))
      (bind _returnvalue (`|SpawnActorFromClass` "/Game/Exam/Blueprints/Inventory/Items/Equipments/Pistol/BP_PistolProjectile.BP_PistolProjectile_C" (`KismetMathLibrary.MakeTransform` _returnvalue_location (`KismetMathLibrary.MakeRotator` 0.0 0.0 _returnvalue_yaw)) "AdjustIfPossibleButAlwaysSpawn" "MultiplyWithRoot" null _aspawn))
      (set `/Game/Exam/Blueprints/Inventory/Items/Equipments/Pistol/BP_PistolProjectile.PistolComponent` self _returnvalue)
      (else
        (`KismetArrayLibrary.Array_RemoveItem` _bulletspool _output)
        (`PrimitiveComponent.SetCollisionEnabled` (`/Game/Exam/Blueprints/Gameplay/BP_Projectile.Sphere` _output) "QueryAndPhysics")
        (set `MovementComponent.Velocity` (1000.0 0.0 0.0) (`/Game/Exam/Blueprints/Gameplay/BP_Projectile.ProjectileMovement` _output))))))